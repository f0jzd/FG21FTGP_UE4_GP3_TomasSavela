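; Player pawn that creates the HUD widget, tracks gamepad use, and fades the camera out on death.
; Input delegates to shoot and dash components and messages the first overlapping interactable through BPI_Interface.
; Shooting, dashing and damage events add montages, dash VFX or positional audio.
; Charge-enemy overlaps on the Box deal damage unless the player is dashing or within a short grace timer counted down on Tick.
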(event OnComponentBeginOverlap(Box)
  (params (OverlappedComponent :type Primitive%20Component%20Object%20Reference) (OtherActor :type Actor%20Object%20Reference) (OtherComp :type Primitive%20Component%20Object%20Reference) (OtherBodyIndex :type Integer) (bFromSweep :type Boolean) (SweepResult :type Hit%20Result%20Structure%20%28by%20ref%29))
  (bind (_asgp3_bpnew_charge_enemy _bsuccess) (Utilities|Casting|CastToGP3_BPNewChargeEnemy OtherActor))
  (if _bsuccess
    (if (not (Variables|/Script/GP3_Team03.GP3DashComponent|GetIsDashing (Variables|Default|GetDashComp)))
      (if (<= (Variables|Default|GetGraceTimer) 0.0)
        (Class|GP3PlayerPawn|RemovePlayerHealth (Variables|/Script/GP3_Team03.GP3_AI_BaseCharacter|GetDamage _asgp3_bpnew_charge_enemy) true)
        (Variables|Default|SetGraceTimer 0.5)))))

(event Custom|TookDamageEvent
  (Animation|Montage|PlayMontage (Variables|Default|GetMeshComp) "/Game/3D_Art/Characters/Sanara/Mixamo_V2/Anims/Sanara_Anim_Standing_React_Small_From_Front_Montage.Sanara_Anim_Standing_React_Small_From_Front_Montage" 3.0
    (:then
      (Class|FMODBlueprintStatics|PlayEventatLocation "/Game/FMOD/Events/SFX_Player/Player_Take_Damage.Player_Take_Damage" (Math|Conversions|ToTransform(Vector) (Transformation|GetActorLocation))))))

(event EventBeginPlay
  (EventDispatchers|BindEventtoTookDamage (delegate Custom|TookDamageEvent))
  (bind _returnvalue (UserInterface|CreateWidget "/Game/Widgets/PlayerWidget.PlayerWidget_C"))
  (bind _output_get (Variables|Default|SetPlayerWidget _returnvalue))
  (UserInterface|Viewport|AddtoViewport _output_get 0))

(event EventOnDashFinish
  ;[1 1 1] Events
  (Components|Activation|Deactivate (Variables|Default|GetDashVFX)))

(event EventTick
  (params (DeltaSeconds :type Float%20%28single-precision%29))
  (if (>= (Variables|Default|GetGraceTimer) 0.0)
    (Variables|Default|SetGraceTimer (- (Variables|Default|GetGraceTimer) DeltaSeconds))))

(event EventOnDashStart
  ;[1 1 1] Events
  (Components|Activation|Activate (Variables|Default|GetDashVFX) true)
  (Class|FMODBlueprintStatics|PlayEventatLocation "/Game/FMOD/Events/SFX_Player/Player_Dash.Player_Dash" (Math|Conversions|ToTransform(Vector) (Transformation|GetActorLocation))))

(event EventOnDeath
  (CameraFades|StartCameraFade :self (Game|GetPlayerCameraManager 0) :ToAlpha 1.0 :Duration 2.0 :bHoldWhenFinished true)
  (Widget|RemovefromParent (Variables|Default|GetPlayerWidget)))

(event Input|ActionEvents|InputActionRestart
  (params (Key :type Key%20Structure :default "None"))
  ;[1 1 1] InputActions
)

(event Input|ActionEvents|InputActionShoot
  (params (Key :type Key%20Structure :default "None"))
  (bind _shootcomp (Variables|Default|GetShootComp))
  ;[1 1 1] InputActions
  (:Pressed
    (Utilities|FlowControl|Sequence
      (:then_0
        (if (and (not (Variables|/Script/GP3_Team03.WeaponBase|GetIsReLoading (Variables|/Script/GP3_Team03.GP3ShootComponent|GetGun _shootcomp))) (Variables|/Script/GP3_Team03.GP3ShootComponent|GetReadyToShoot _shootcomp))
          (Animation|Montage|PlayMontage (Variables|Default|GetMeshComp) "/Game/3D_Art/Characters/Sanara/Mixamo_V2/Anims/Sanara_Anim_Standing_1H_Magic_Attack_01_Montage.Sanara_Anim_Standing_1H_Magic_Attack_01_Montage" 2.5 1.0
            (:then
              (Class|FMODBlueprintStatics|PlayEventatLocation "/Game/FMOD/Events/SFX_Player/Player_Shoot.Player_Shoot" (Math|Conversions|ToTransform(Vector) (Transformation|GetActorLocation)))))))
      (:then_1
        (Class|GP3ShootComponent|Shoot _shootcomp)))))

(event Input|ActionEvents|InputActionDash
  (params (Key :type Key%20Structure :default "None"))
  ;[1 1 1] InputActions
  (:Pressed
    (Class|GP3DashComponent|Dash (Variables|Default|GetDashComp) (Variables|Default|GetForwardInputValue) (Variables|Default|GetRightInputValue))))

(event Input|ActionEvents|InputActionInteract
  (params (Key :type Key%20Structure :default "None"))
  ;[1 1 1] InputActions
  (:Pressed
    (bind _array_element (Utilities|Array|ForEachLoopwithBreak (Collision|GetOverlappingActors "/Game/Blueprints/Gameplay/BP_InteractableObject.BP_InteractableObject_C" :!class /Script/Engine.Actor) :!label _label)
      (:LoopBody
        (if (Utilities|DoesObjectImplementInterface _array_element "/Game/Blueprints/Gameplay/BPI_Interface.BPI_Interface_C")
          (Class|BPIInterface|Interact(Message) _array_element)
          (goto _label Break))))))

(event Input|ActionEvents|InputActionDodge
  (params (Key :type Key%20Structure :default "None"))
  ;[1 1 1] old dodge
)

(event Input|KeyboardEvents|AnyKey
  (params (Key :type Key%20Structure :default "None"))
  (:Pressed
    (Variables|Default|SetbIsUsingGamepad (Class|KismetInputLibrary|KeyIsGamepadKey Key))))

(fn ConstructionScript)