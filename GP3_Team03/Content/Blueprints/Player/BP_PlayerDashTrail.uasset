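; BP_PlayerDashTrail is an actor that builds a trail along a spline, named for the player's dash.
; OnSpawn adds the first spline point, and each OnExtendSpline call appends another at the given location.
; Each extension also creates a manually attached, X-forward spline mesh spanning the previous point to the given index, using the spline's world-space positions and tangents.
; Points are added in local space but read back in world space.
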(event EventOnSpawn
  (params (Location :type Vector :default "0, 0, 0"))
  (Spline|AddSplinePoint (Variables|Default|GetSpline) Location "Local" true))

(event EventOnExtendSpline
  (params (Index :type Integer) (Location :type Vector :default "0, 0, 0"))
  (bind _returnvalue (- Index 1))
  (bind _spline (Variables|Default|GetSpline))
  (bind _spline_2 (Variables|Default|GetSpline))
  (Spline|AddSplinePoint (Variables|Default|GetSpline) Location "Local" true)
  (bind _returnvalue_2 (AddComponent|AddSplineMeshComponent true))
  (SplineMesh|SetForwardAxis _returnvalue_2 "X" true)
  (SplineMesh|SetStartandEnd _returnvalue_2 (Spline|GetLocationatSplinePoint _spline _returnvalue "World") (Spline|GetTangentatSplinePoint _spline _returnvalue "World") (Spline|GetLocationatSplinePoint _spline_2 Index "World") (Spline|GetTangentatSplinePoint _spline_2 Index "World") true :!class /Script/Engine.SplineMeshComponent))

(fn ConstructionScript)