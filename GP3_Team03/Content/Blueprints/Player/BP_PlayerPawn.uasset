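; Player pawn that creates the pause menu and crosshair widgets on begin play and routes player actions to its components.
; Each tick it passes stored forward and right input values to WASDMovementComp for movement.
; The Shoot action calls ShootComp, while the Restart action opens a hard-referenced test level, OssiansTestLevel.
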(event EventBeginPlay
  (bind _returnvalue (UserInterface|CreateWidget "/Game/Widgets/PauseMenuWidget.PauseMenuWidget_C"))
  (UserInterface|Viewport|AddtoViewport _returnvalue 5)
  (bind _returnvalue_2 (UserInterface|CreateWidget "/Game/Widgets/CrosshairWidget.CrosshairWidget_C"))
  (UserInterface|Viewport|AddtoViewport _returnvalue_2 0))

(event EventTick
  (params (DeltaSeconds :type Float%20%28single-precision%29))
  (Class|GP3WASDMovementComponent|Move (Variables|Default|GetWASDMovementComp) (Variables|Default|GetForwardInputValue) (Variables|Default|GetRightInputValue) DeltaSeconds))

(event Input|ActionEvents|InputActionRestart
  (params (Key :type Key%20Structure :default "None"))
  (:Pressed
    (Game|OpenLevel(byObjectReference) "/Game/Maps/OssiansTestLevels/OssiansTestLevel.OssiansTestLevel")))

(event Input|ActionEvents|InputActionShoot
  (params (Key :type Key%20Structure :default "None"))
  (:Pressed
    (Class|GP3ShootComponent|Shoot (Variables|Default|GetShootComp))))

(fn ConstructionScript)