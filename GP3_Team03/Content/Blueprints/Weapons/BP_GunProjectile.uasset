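; Gun projectile with an attached fireball effect that damages charge and ranged enemies.
; On spawn it sets a fixed local-space velocity, angled slightly off forward.
; On collision it casts the hit actor to each enemy type, applies damage, then always destroys itself.
; Hits on a debuffed enemy's WeakSpot-tagged component deal critical damage, but only charge enemies also fire the OnWeakPointHit dispatcher.
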(event OnComponentHit(Mesh)
  (params (HitComponent :type Primitive%20Component%20Object%20Reference) (OtherActor :type Actor%20Object%20Reference) (OtherComp :type Primitive%20Component%20Object%20Reference) (NormalImpulse :type Vector :default "0, 0, 0") (Hit :type Hit%20Result%20Structure%20%28by%20ref%29)))

(event OnComponentHit(Collision)
  (params (HitComponent :type Primitive%20Component%20Object%20Reference) (OtherActor :type Actor%20Object%20Reference) (OtherComp :type Primitive%20Component%20Object%20Reference) (NormalImpulse :type Vector :default "0, 0, 0") (Hit :type Hit%20Result%20Structure%20%28by%20ref%29))
  (bind (_asgp3bp_ranged_enemy_character _bsuccess) (Utilities|Casting|CastToGP3BP_RangedEnemyCharacter OtherActor))
  (bind (_asgp3_bpnew_charge_enemy _bsuccess_2) (Utilities|Casting|CastToGP3_BPNewChargeEnemy OtherActor))
  ;[1 1 1] Check to see what we hit, if its a charge enemy, call charge enemy function, if its a ranged enemy, ranged enemy function, and destroy itself in the end no matter the outcome
  (if _bsuccess_2
    (CallFunction|DamageChargeEnemy _asgp3_bpnew_charge_enemy OtherComp)
    (elif _bsuccess
      (CallFunction|DamageRangedEnemy _asgp3bp_ranged_enemy_character OtherComp)))
  (Actor|DestroyActor))

(event EventBeginPlay
  (bind _scene (Variables|Default|GetScene))
  (Niagara|SpawnSystemAttached "/Game/3D_Art/Characters/Sanara_VFX/Cast_Fire_Ball/Fire_Ball.Fire_Ball" _scene "None" (Variables|/Script/Engine.SceneComponent|GetRelativeLocation _scene) (Variables|/Script/Engine.SceneComponent|GetRelativeRotation _scene) "KeepRelativeOffset" false)
  (Game|Components|ProjectileMovement|SetVelocityinLocalSpace (Variables|Default|GetProjectileComponent) "3500.000000,40.000000,225.000000"))

(fn ConstructionScript)

(fn DamageChargeEnemy
  (params (ChargEnemyRef :type GP3%20BP%20New%20Charge%20Enemy%20Object%20Reference) (HitComponent :type Primitive%20Component%20Object%20Reference))
  (if (and (Variables|/Script/GP3_Team03.GP3_AI_BaseCharacter|GetIsDebuffed ChargEnemyRef) (Components|ComponentHasTag HitComponent "WeakSpot"))
    (Default|CallOnWeakPointHit)
    (Default|CriticalDamage ChargEnemyRef)
    (Class|GP3AIBaseCharacter|TakeGunDamage ChargEnemyRef (Variables|Default|GetCriticalDamage))
    (else
      (Class|GP3AIBaseCharacter|TakeGunDamage ChargEnemyRef (Variables|Default|GetDamage)))))

(fn DamageRangedEnemy
  (params (RangedEnemyRef :type GP3%20Ranged%20Enemy%20Character%20Object%20Reference) (Hit%20Component :type Primitive%20Component%20Object%20Reference))
  (bind _asgp3bp_ranged_enemy_character (Utilities|Casting|CastToGP3BP_RangedEnemyCharacter RangedEnemyRef))
  (if (Utilities|IsValid RangedEnemyRef)
    (if (and (Variables|/Script/GP3_Team03.GP3_AI_BaseCharacter|GetIsDebuffed RangedEnemyRef) (Components|ComponentHasTag Hit%20Component "WeakSpot"))
      (Default|CriticalDamage _asgp3bp_ranged_enemy_character)
      (Class|GP3AIBaseCharacter|TakeGunDamage RangedEnemyRef (Variables|Default|GetCriticalDamage))
      (else
        (Class|GP3AIBaseCharacter|TakeGunDamage _asgp3bp_ranged_enemy_character (Variables|Default|GetDamage))))
    (else
      (return))))