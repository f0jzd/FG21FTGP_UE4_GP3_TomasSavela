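; GP3SettingsGameInstance is a game instance that owns the player's settings save data for the lifetime of the game.
; On Init it loads the SettingsSaveGame from its save slot, or creates a fresh one if none exists or the cast fails.
; It exposes the object through GetSettingsSaveGame and writes it back to the slot on Shutdown.
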(event EventShutdown
  (SaveGame|SaveGametoSlot (Variables|Default|GetSettingsData) (Variables|Default|GetSaveGameName)))

(event EventInit
  (bind _returnvalue (SaveGame|DoesSaveGameExist (Variables|Default|GetSaveGameName)))
  (if _returnvalue
    (bind _returnvalue_2 (SaveGame|LoadGamefromSlot (Variables|Default|GetSaveGameName)))
    (bind _assettings_save_game (Utilities|Casting|CastToSettingsSaveGame _returnvalue_2)
      (:then
        (Variables|Default|SetSettingsData _assettings_save_game))
      (:CastFailed
        (bind _returnvalue_3 (SaveGame|CreateSaveGameObject "/Game/Data/SettingsSaveGame.SettingsSaveGame_C" :!label _label))
        (Variables|Default|SetSettingsData _returnvalue_3)))
    (else
      (goto _label))))

(fn GetSettingsSaveGame
  (return (Variables|Default|GetSettingsData)))