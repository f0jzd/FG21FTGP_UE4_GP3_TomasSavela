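; Tutorial trigger volume that shows a control-prompt widget when the player pawn overlaps it, or when its PlayAnimation event is called.
; The widget appears with a reversed dissolve, which AnimationNumber selects for overlaps.
; Tick swaps move, look, shoot, aim and dash icons between gamepad and keyboard/mouse.
; End overlap plays the dissolve forward, removes the widget and clears Condition, disabling further overlap triggers.
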(event OnComponentBeginOverlap(TriggerBox)
  (params (OverlappedComponent :type Primitive%20Component%20Object%20Reference) (OtherActor :type Actor%20Object%20Reference) (OtherComp :type Primitive%20Component%20Object%20Reference) (OtherBodyIndex :type Integer) (bFromSweep :type Boolean) (SweepResult :type Hit%20Result%20Structure%20%28by%20ref%29))
  (bind _show_widget_animation (Variables|Default|GetShow%20Widget%20Animation))
  (if (Variables|Default|GetCondition)
    (if (== (Game|Player|GetPlayerPawn 0) OtherActor)
      (bind _returnvalue (UserInterface|CreateWidget "/Game/Widgets/TutorialWidget.TutorialWidget_C"))
      (Variables|Default|SetWidget _returnvalue)
      (Utilities|Array|Add _show_widget_animation (Variables|/Game/Widgets/TutorialWidget.TutorialWidget_C|GetDissolve _returnvalue))
      (Utilities|Array|Add _show_widget_animation (Variables|/Game/Widgets/TutorialWidget.TutorialWidget_C|GetDissolve2 _returnvalue))
      (Utilities|Array|Add _show_widget_animation (Variables|/Game/Widgets/TutorialWidget.TutorialWidget_C|GetDissolve3 _returnvalue))
      (UserInterface|Viewport|AddtoViewport _returnvalue 0)
      (UserInterface|Animation|PlayAnimation _returnvalue (Utilities|Array|Get(acopy) _show_widget_animation (Variables|Default|GetAnimation%20Number)) 0.0 1 "Reverse" 2.0 false))))

(event OnComponentEndOverlap(TriggerBox)
  (params (OverlappedComponent :type Primitive%20Component%20Object%20Reference) (OtherActor :type Actor%20Object%20Reference) (OtherComp :type Primitive%20Component%20Object%20Reference) (OtherBodyIndex :type Integer))
  (bind _widget (Variables|Default|GetWidget))
  (if (Variables|Default|GetCondition)
    (Utilities|FlowControl|Sequence
      (:then_0
        (if (Utilities|IsValid _widget)
          (Components|Animation|PlayAnimation _widget (Variables|/Game/Widgets/TutorialWidget.TutorialWidget_C|GetDissolve _widget) 0.0
            (:Finished
              (Widget|RemovefromParent _widget)
              (Variables|Default|SetCondition false)))))
      (:then_1
        (Components|Animation|PlayAnimation (Variables|Default|GetWidget) (Utilities|Array|Get(acopy) (Variables|Default|GetShow%20Widget%20Animation) (Variables|Default|GetAnimation%20Number)) 0.0
          (:Finished
            (Widget|RemovefromParent (stale OnComponentBeginOverlap(TriggerBox) _returnvalue))
            (Variables|Default|SetCondition false)))))))

(event Custom|PlayAnimation
  (bind _returnvalue (UserInterface|CreateWidget "/Game/Widgets/TutorialWidget.TutorialWidget_C"))
  (bind _output_get (Variables|Default|SetWidget _returnvalue))
  (UserInterface|Viewport|AddtoViewport _output_get 0)
  (UserInterface|Animation|PlayAnimation (Variables|Default|GetWidget) (Variables|/Game/Widgets/TutorialWidget.TutorialWidget_C|GetDissolve (Variables|Default|GetWidget)) 0.0 1 "Reverse" 2.0 false))

(event EventTick
  (params (DeltaSeconds :type Float%20%28single-precision%29))
  (bind _widget (Variables|Default|GetWidget))
  (bind _widget_2 (Variables|Default|GetWidget))
  (if (Utilities|IsValid (stale Custom|PlayAnimation _output_get))
    (bind _asbp_player_pawnv_2 (Utilities|Casting|CastToBP_PlayerPawnv2 (Game|Player|GetPlayerPawn 0)))
    (if (Variables|/Script/GP3_Team03.GP3PlayerPawn|GetbIsUsingGamepad _asbp_player_pawnv_2)
      (bind _output_get (Variables|/Game/Widgets/TutorialWidget.TutorialWidget_C|SetMove%20Texture _widget_2 (Variables|Default|GetL%20Stick)))
      (Default|GetMoveIcon _widget_2 _output_get)
      (bind _output_get_2 (Variables|/Game/Widgets/TutorialWidget.TutorialWidget_C|SetLook%20Texture _widget_2 (Variables|Default|GetR%20Stick)))
      (Default|GetLookIcon _widget_2 _output_get_2)
      (bind _output_get_3 (Variables|/Game/Widgets/TutorialWidget.TutorialWidget_C|SetShoot%20Texture _widget_2 (Variables|Default|GetRT)))
      (Default|GetShootIcon _widget_2 _output_get_3)
      (bind _output_get_4 (Variables|/Game/Widgets/TutorialWidget.TutorialWidget_C|SetAim%20Texture _widget_2 (Variables|Default|GetLT)))
      (Default|GetAimIcon _widget_2 _output_get_4)
      (bind _output_get_5 (Variables|/Game/Widgets/TutorialWidget.TutorialWidget_C|SetDash%20Texture _widget_2 (Variables|Default|GetLB)))
      (Default|GetDashIcon _widget_2 _output_get_5)
      (else
        (bind _output_get_6 (Variables|/Game/Widgets/TutorialWidget.TutorialWidget_C|SetMove%20Texture _widget (Variables|Default|GetWASD)))
        (Default|GetMoveIcon _widget _output_get_6)
        (bind _output_get_7 (Variables|/Game/Widgets/TutorialWidget.TutorialWidget_C|SetLook%20Texture _widget (Variables|Default|GetMouse)))
        (Default|GetLookIcon _widget _output_get_7)
        (bind _output_get_8 (Variables|/Game/Widgets/TutorialWidget.TutorialWidget_C|SetShoot%20Texture _widget (Variables|Default|GetLeft%20Click)))
        (Default|GetShootIcon _widget _output_get_8)
        (bind _output_get_9 (Variables|/Game/Widgets/TutorialWidget.TutorialWidget_C|SetAim%20Texture _widget (Variables|Default|GetRight%20Click)))
        (Default|GetAimIcon _widget _output_get_9)
        (bind _output_get_10 (Variables|/Game/Widgets/TutorialWidget.TutorialWidget_C|SetDash%20Texture _widget (Variables|Default|GetShift)))
        (Default|GetDashIcon _widget _output_get_10)))))

(fn ConstructionScript)