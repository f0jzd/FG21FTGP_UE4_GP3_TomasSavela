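; Wave-based enemy spawn trigger that runs an arena encounter from a DT_WaveInfo row.
; Tick spawns each wave through EnemySpawner when it is active and ready, registering enemies in GM_GP3.
; Once none remain valid (CheckIfEnemiesLeft returns true when empty), it restarts the spawner timer.
; After the final wave, it enables the end-level arena trigger, hiding ShadowGate, or interactable object, then switches the music.
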(event EventBeginPlay
  (bind _returnvalue (Utilities|GetDataTableRow "/Game/Data/DT_WaveInfo.DT_WaveInfo" (Variables|Publics|GetWaveSettingsRowName))
    (:then
      (bind _output_get (Variables|Default|SetWaveSettings _returnvalue))
      (Variables|Default|SetCurrentWaveNumber 0)
      (Variables|Default|SetMaxWaveAmount (Utilities|Array|LastIndex (Utilities|Struct|BreakS_WaveInfo _output_get))))))

(event EventTick
  (params (DeltaSeconds :type Float%20%28single-precision%29))
  (bind _shadowgate (Variables|Default|GetShadowGate))
  (bind _endlevelsequencetrigger (Variables|Publics|GetEndLevelSequenceTrigger))
  (bind _enemyspawner (Variables|Default|GetEnemySpawner))
  (if (Variables|/Script/GP3_Team03.SpawningEnemySystem|GetbSpawnerActivated _enemyspawner)
    (if (Variables|/Script/GP3_Team03.SpawningEnemySystem|GetbReadyToSpawn _enemyspawner)
      (CallFunction|SpawnWave)
      (Class|FMODBlueprintStatics|PlayEvent2D "/Game/FMOD/Events/SFX_Enemy/Enemy_Spawning.Enemy_Spawning")
      (bind _result (Math|Integer|IncrementInt (Variables|Default|GetCurrentWaveNumber))
        (:%20%20
          (Variables|Default|SetCurrentWaveNumber _result)
          (Variables|/Script/GP3_Team03.SpawningEnemySystem|SetbReadyToSpawn (Variables|Default|GetEnemySpawner) false)
          (if (> (Variables|Default|GetCurrentWaveNumber) (Variables|Default|GetMaxWaveAmount))
            (Variables|Default|SetFinalWaveSpawned true))))
      (else
        (bind _all_enemies_defeated (CallFunction|CheckifEnemiesLeft))
        (if _all_enemies_defeated
          (if (Variables|Default|GetFinalWaveSpawned)
            (bind _asbp_arena_trigger (Utilities|Casting|CastToBP_ArenaTrigger _endlevelsequencetrigger)
              (:then
                (Variables|/Game/Blueprints/Gameplay/BP_ArenaTrigger.BP_ArenaTrigger_C|SetShouldTrigger _asbp_arena_trigger true)
                (if (Utilities|IsValid _shadowgate)
                  (Collision|SetCollisionEnabled (Variables|/Script/Engine.StaticMeshActor|GetStaticMeshComponent _shadowgate) "NoCollision")
                  (Rendering|SetActorHiddenInGame _shadowgate true)
                  (if (not (Variables|Default|GetEndAudioPlayed)) :!label _label
                    (Class|FMODBlueprintStatics|BusStopAllEvents "/Game/FMOD/Buses/Master/Music.Music" "ALLOWFADEOUT")
                    (bind _returnvalue (Class|FMODBlueprintStatics|PlayEventAttached "/Game/FMOD/Events/Music/Press_Play.Press_Play" (Variables|/Script/Engine.PlayerCameraManager|GetTransformComponent (Game|GetPlayerCameraManager 0)) "None" "0, 0, 0" "KeepRelativeOffset"))
                    (Class|FMODAudioComponent|SetParameter _returnvalue "Progress" 1.0)
                    (Variables|Default|SetEndAudioPlayed true))))
              (:CastFailed
                (bind _asbp_interactable_object (Utilities|Casting|CastToBP_InteractableObject _endlevelsequencetrigger))
                (Variables|/Game/Blueprints/Gameplay/BP_InteractableObject.BP_InteractableObject_C|SetIsInteractable _asbp_interactable_object true)
                (goto _label)))
            (else
              (Variables|/Script/GP3_Team03.SpawningEnemySystem|SetbTimerIsOn (Variables|Default|GetEnemySpawner) true))))))))

(fn ConstructionScript)

(fn SpawnWave
  (bind _currentwavenumber (Variables|Default|GetCurrentWaveNumber))
  (bind _wavesettings (Variables|Default|GetWaveSettings))
  (bind _waveinfo (Utilities|Struct|BreakS_WaveInfo _wavesettings))
  (bind _output (Utilities|Array|Get(acopy) _waveinfo _currentwavenumber))
  (bind (_enemyclasses _amounttospawn) (Utilities|Struct|BreakS_WaveEnemyInfo _output))
  (for (_array_element _array_index) _enemyclasses
    (for _index (range 1 (Utilities|Array|Get(acopy) _amounttospawn _array_index))
      (bind _spawnedenemy (Class|SpawningEnemySystem|SpawnEnemy (Variables|Default|GetEnemySpawner) _array_element))
      (bind _asgm_gp3 (Utilities|Casting|CastToGM_GP3 (Game|GetGameMode)))
      (bind _output_get (Variables|/Game/Blueprints/GameMode/GM_GP3.GM_GP3_C|SetActiveEnemiesInLevel _asgm_gp3 (Variables|/Game/Blueprints/GameMode/GM_GP3.GM_GP3_C|GetActiveEnemiesInLevel _asgm_gp3)))
      (Utilities|Array|Add _output_get _spawnedenemy)))
  (return))

(fn CheckifEnemiesLeft
  (bind _asgm_gp3 (Utilities|Casting|CastToGM_GP3 (Game|GetGameMode)))
  (for _array_element (Variables|/Game/Blueprints/GameMode/GM_GP3.GM_GP3_C|GetActiveEnemiesInLevel _asgm_gp3)
    (Utilities|IsValid _array_element
      (:Is%20Valid
        (return false))))
  (return true))