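; Trigger volume that shows a movement and look tutorial widget while something overlaps its box.
; Begin overlap, or the PlayAnimation event, creates the widget, reveals it by playing its Dissolve animation in reverse and enables Tick.
; Tick swaps the move and look textures between gamepad sticks and WASD/mouse based on the player pawn's input device.
; End overlap plays Dissolve forward and disables Tick.
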(event OnComponentBeginOverlap(Triggerbox)
  (params (OverlappedComponent :type Primitive%20Component%20Object%20Reference) (OtherActor :type Actor%20Object%20Reference) (OtherComp :type Primitive%20Component%20Object%20Reference) (OtherBodyIndex :type Integer) (bFromSweep :type Boolean) (SweepResult :type Hit%20Result%20Structure%20%28by%20ref%29))
  (bind _returnvalue (UserInterface|CreateWidget "/Game/Widgets/TutorialMoveWidget.TutorialMoveWidget_C"))
  (bind _output_get (Variables|Default|SetWidget _returnvalue))
  (UserInterface|Viewport|AddtoViewport _output_get 0)
  (UserInterface|Animation|PlayAnimation _output_get (Variables|/Game/Widgets/TutorialMoveWidget.TutorialMoveWidget_C|GetDissolve _output_get) 0.0 1 "Reverse" 1.0 false)
  (Actor|Tick|SetActorTickEnabled true))

(event OnComponentEndOverlap(Triggerbox)
  (params (OverlappedComponent :type Primitive%20Component%20Object%20Reference) (OtherActor :type Actor%20Object%20Reference) (OtherComp :type Primitive%20Component%20Object%20Reference) (OtherBodyIndex :type Integer))
  (bind _widget (Variables|Default|GetWidget))
  (if (Utilities|IsValid (Variables|Default|GetWidget))
    (UserInterface|Animation|PlayAnimation _widget (Variables|/Game/Widgets/TutorialMoveWidget.TutorialMoveWidget_C|GetDissolve _widget) 0.0 1 "Forward" 1.0 false)
    (Actor|Tick|SetActorTickEnabled false)))

(event Custom|PlayAnimation
  (bind _returnvalue (UserInterface|CreateWidget "/Game/Widgets/TutorialMoveWidget.TutorialMoveWidget_C"))
  (bind _output_get (Variables|Default|SetWidget _returnvalue))
  (UserInterface|Viewport|AddtoViewport _output_get 0)
  (UserInterface|Animation|PlayAnimation _output_get (Variables|/Game/Widgets/TutorialMoveWidget.TutorialMoveWidget_C|GetDissolve _output_get) 0.0 1 "Reverse" 1.0 false)
  (Actor|Tick|SetActorTickEnabled true))

(event EventBeginPlay
  (Actor|Tick|SetActorTickEnabled false))

(event EventTick
  (params (DeltaSeconds :type Float%20%28single-precision%29))
  (bind _widget (Variables|Default|GetWidget))
  (bind _widget_2 (Variables|Default|GetWidget))
  (if (Utilities|IsValid (Variables|Default|GetWidget))
    (bind _asbp_player_pawnv_2 (Utilities|Casting|CastToBP_PlayerPawnv2 (Game|Player|GetPlayerPawn 0)))
    (if (Variables|/Script/GP3_Team03.GP3PlayerPawn|GetbIsUsingGamepad _asbp_player_pawnv_2)
      (Variables|/Game/Widgets/TutorialMoveWidget.TutorialMoveWidget_C|SetMove%20Texture _widget_2 (Variables|Default|GetL%20Stick))
      (Variables|/Game/Widgets/TutorialMoveWidget.TutorialMoveWidget_C|SetLook%20Texture _widget_2 (Variables|Default|GetR%20Stick))
      (else
        (Variables|/Game/Widgets/TutorialMoveWidget.TutorialMoveWidget_C|SetMove%20Texture _widget (Variables|Default|GetWASD))
        (Variables|/Game/Widgets/TutorialMoveWidget.TutorialMoveWidget_C|SetLook%20Texture _widget (Variables|Default|GetMouse))))))

(fn ConstructionScript)