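; Sequence Director logic for the Level 1 intro sequence, holding the events the Sequencer fires during the intro.
; One event disables player pawn input, then after a short delay hides the player widget and blocks pausing.
; A second event restores input, widget visibility and pausing through the pawn reference cast in the first.
; A third event plays the animation on a movement tutorial trigger passed in from the sequence.
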(event Custom|SequenceEvent_0
  (bind _returnvalue (Game|Player|GetPlayerPawn 0))
  (Input|DisableInput _returnvalue 0)
  (Utilities|FlowControl|Delay 0.1)
  (bind _asbp_player_pawnv_2 (Utilities|Casting|CastToBP_PlayerPawnv2 _returnvalue))
  (Widget|SetVisibility (Variables|/Game/Blueprints/Player/BP_PlayerPawnv2.BP_PlayerPawnv2_C|GetPlayerWidget _asbp_player_pawnv_2) "Hidden")
  (Variables|/Game/Widgets/PauseMenuWidget.PauseMenuWidget_C|SetCanPause (Variables|/Game/Widgets/PlayerWidget.PlayerWidget_C|GetPauseMenuWidget (Variables|/Game/Blueprints/Player/BP_PlayerPawnv2.BP_PlayerPawnv2_C|GetPlayerWidget _asbp_player_pawnv_2)) false))

(event Custom|SequenceEvent_1
  (Input|EnableInput (Game|Player|GetPlayerPawn 0) 0)
  (Widget|SetVisibility (Variables|/Game/Blueprints/Player/BP_PlayerPawnv2.BP_PlayerPawnv2_C|GetPlayerWidget (stale Custom|SequenceEvent_0 _asbp_player_pawnv_2)) "Visible")
  (Variables|/Game/Widgets/PauseMenuWidget.PauseMenuWidget_C|SetCanPause (Variables|/Game/Widgets/PlayerWidget.PlayerWidget_C|GetPauseMenuWidget (Variables|/Game/Blueprints/Player/BP_PlayerPawnv2.BP_PlayerPawnv2_C|GetPlayerWidget (stale Custom|SequenceEvent_0 _asbp_player_pawnv_2))) true))

(event Custom|SequenceEvent_2
  (params (Move%20Tutorial%20Trigger :type BP%20Move%20Tutorial%20Trigger%20Object%20Reference))
  (Default|PlayAnimation Move%20Tutorial%20Trigger))