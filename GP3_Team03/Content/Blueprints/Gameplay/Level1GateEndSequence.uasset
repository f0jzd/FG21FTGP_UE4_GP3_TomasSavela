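; Sequence director for the Level 1 gate end cinematic, with events that handle the player, audio and level transition.
; One event disables pawn input, then hides the player widget and blocks pausing after a short delay.
; Another opens LevelToLoad by object reference if valid, and a third plays the Clearing_First_Area 2D audio event after a delay.
; The logic to restore input and UI and the debug prints are unconnected.
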(event Custom|SequenceEvent_0
  (bind _returnvalue (Game|Player|GetPlayerPawn 0))
  (Input|DisableInput _returnvalue 0)
  (Utilities|FlowControl|Delay 0.1)
  (bind _asbp_player_pawnv_2 (Utilities|Casting|CastToBP_PlayerPawnv2 _returnvalue))
  (Widget|SetVisibility (Variables|/Game/Blueprints/Player/BP_PlayerPawnv2.BP_PlayerPawnv2_C|GetPlayerWidget _asbp_player_pawnv_2) "Hidden")
  (Variables|/Game/Widgets/PauseMenuWidget.PauseMenuWidget_C|SetCanPause (Variables|/Game/Widgets/PlayerWidget.PlayerWidget_C|GetPauseMenuWidget (Variables|/Game/Blueprints/Player/BP_PlayerPawnv2.BP_PlayerPawnv2_C|GetPlayerWidget _asbp_player_pawnv_2)) false))

(event Custom|SequenceEvent_1
  (bind _leveltoload (Variables|Default|GetLevelToLoad)
    (:then
      (Game|OpenLevel(byObjectReference) _leveltoload))
    (:else)))

(event Custom|SequenceEvent_2
  (Utilities|FlowControl|Delay 1.0)
  (Class|FMODBlueprintStatics|PlayEvent2D "/Game/FMOD/Events/Music/Clearing_First_Area.Clearing_First_Area"))