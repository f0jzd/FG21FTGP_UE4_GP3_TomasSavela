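; Sequence event Blueprint for the Level 1 Shadow Gate cinematic, handling player lockout, spawner activation and portal audio.
; One event disables input, then after a short delay hides the player widget and blocks pausing; a second event restores all three.
; Other events arm a passed-in enemy spawner and play the Shadow_Gate sound at the camera location.
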(event Custom|event0
  (bind _returnvalue (Game|Player|GetPlayerPawn 0))
  (Input|DisableInput _returnvalue 0)
  (Utilities|FlowControl|Delay 0.1)
  (bind _asbp_player_pawnv_2 (Utilities|Casting|CastToBP_PlayerPawnv2 _returnvalue))
  (Widget|SetVisibility (Variables|/Game/Blueprints/Player/BP_PlayerPawnv2.BP_PlayerPawnv2_C|GetPlayerWidget _asbp_player_pawnv_2) "Hidden")
  (Variables|/Game/Widgets/PauseMenuWidget.PauseMenuWidget_C|SetCanPause (Variables|/Game/Widgets/PlayerWidget.PlayerWidget_C|GetPauseMenuWidget (Variables|/Game/Blueprints/Player/BP_PlayerPawnv2.BP_PlayerPawnv2_C|GetPlayerWidget _asbp_player_pawnv_2)) false))

(event Custom|event1
  (Input|EnableInput (Game|Player|GetPlayerPawn 0) 0)
  (Widget|SetVisibility (Variables|/Game/Blueprints/Player/BP_PlayerPawnv2.BP_PlayerPawnv2_C|GetPlayerWidget (stale Custom|event0 _asbp_player_pawnv_2)) "Visible")
  (Variables|/Game/Widgets/PauseMenuWidget.PauseMenuWidget_C|SetCanPause (Variables|/Game/Widgets/PlayerWidget.PlayerWidget_C|GetPauseMenuWidget (Variables|/Game/Blueprints/Player/BP_PlayerPawnv2.BP_PlayerPawnv2_C|GetPlayerWidget (stale Custom|event0 _asbp_player_pawnv_2))) true))

(event Custom|play%20portal%20sound
  (Class|FMODBlueprintStatics|PlayEventatLocation "/Game/FMOD/Events/SFX_Environment/Shadow_Gate.Shadow_Gate" (Math|Conversions|ToTransform(Vector) (Camera|GetCameraLocation (Game|GetPlayerCameraManager 0)))))

(event Custom|SequenceEvent_0
  (params (EnemySpawner :type Spawning%20Enemy%20System%20Object%20Reference))
  (Development|PrintString "Sequnce ran")
  (Variables|Default|SetEnemySpawner EnemySpawner)
  (bind _enemyspawner (Variables|Default|GetEnemySpawner)
    (:then
      (Variables|/Script/GP3_Team03.SpawningEnemySystem|SetbSpawnerActivated _enemyspawner true)
      (Variables|/Script/GP3_Team03.SpawningEnemySystem|SetbReadyToSpawn _enemyspawner true))
    (:else)))