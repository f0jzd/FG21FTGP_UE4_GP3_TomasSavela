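; BP_ArenaTrigger is a one-shot trigger actor that plays a Level Sequence when the player pawn enters it.
; While ShouldTrigger is set, Tick polls for player overlap; the component's begin-overlap event is empty and its older logic is disconnected.
; On firing, it fades out the Music bus and plays an optional audio event attached to the camera manager.
; It then starts the sequence, disables trigger overlaps and sets SequenceTriggered.
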(event OnComponentBeginOverlap(LevelSequenceTrigger)
  (params (OverlappedComponent :type Primitive%20Component%20Object%20Reference) (OtherActor :type Actor%20Object%20Reference) (OtherComp :type Primitive%20Component%20Object%20Reference) (OtherBodyIndex :type Integer) (bFromSweep :type Boolean) (SweepResult :type Hit%20Result%20Structure%20%28by%20ref%29)))

(event EventTick
  (params (DeltaSeconds :type Float%20%28single-precision%29))
  (bind _audioeventtoplay (Variables|Default|GetAudioEventToPlay))
  (if (Variables|Default|GetShouldTrigger)
    (if (not (Variables|Default|GetSequenceTriggered))
      (if (Collision|IsOverlappingActor (Game|Player|GetPlayerPawn 0) :!class /Script/Engine.Actor)
        (if (Utilities|IsValid _audioeventtoplay)
          (Class|FMODBlueprintStatics|BusStopAllEvents "/Game/FMOD/Buses/Master/Music.Music" "ALLOWFADEOUT")
          (Class|FMODBlueprintStatics|PlayEventAttached _audioeventtoplay (Variables|/Script/Engine.PlayerCameraManager|GetTransformComponent (Game|GetPlayerCameraManager 0)) "None" "0, 0, 0" "KeepRelativeOffset"))
        (bind _outactor (Sequencer|Player|CreateLevelSequencePlayer (Variables|Default|GetLevel%20Sequence)))
        (Sequencer|Player|Play (Variables|/Script/LevelSequence.LevelSequenceActor|GetSequencePlayer _outactor) :!class /Script/MovieScene.MovieSceneSequencePlayer)
        (Variables|/Script/Engine.PrimitiveComponent|SetbGenerateOverlapEvents (Variables|Default|GetLevelSequenceTrigger) false)
        (Variables|Default|SetSequenceTriggered true)))))

(fn ConstructionScript)