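; Interactable world object that plays a level sequence when triggered through Interact, provided it is flagged interactable.
; Its trigger volume shows an interact prompt while the player pawn overlaps, enabling Tick only then to swap keyboard and Xbox icons by active input.
; Interact removes the prompt, starts the sequence and, if an audio event is set, immediately fades out the Music bus and plays that event on the camera manager.
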(event OnComponentBeginOverlap(InteractTrigger)
  (params (OverlappedComponent :type Primitive%20Component%20Object%20Reference) (OtherActor :type Actor%20Object%20Reference) (OtherComp :type Primitive%20Component%20Object%20Reference) (OtherBodyIndex :type Integer) (bFromSweep :type Boolean) (SweepResult :type Hit%20Result%20Structure%20%28by%20ref%29))
  (if (and (Variables|Default|GetIsInteractable) (== OtherActor (Game|Player|GetPlayerPawn 0)))
    (bind _returnvalue (UserInterface|CreateWidget "/Game/Blueprints/Gameplay/BPWidget_Interact.BPWidget_Interact_C"))
    (bind _output_get (Variables|Default|SetWidget _returnvalue))
    (UserInterface|Viewport|AddtoViewport _returnvalue 0)
    (Actor|Tick|SetActorTickEnabled true)))

(event OnComponentEndOverlap(InteractTrigger)
  (params (OverlappedComponent :type Primitive%20Component%20Object%20Reference) (OtherActor :type Actor%20Object%20Reference) (OtherComp :type Primitive%20Component%20Object%20Reference) (OtherBodyIndex :type Integer))
  (if (and (Variables|Default|GetIsInteractable) (== OtherActor (Game|Player|GetPlayerPawn 0)))
    (Widget|RemovefromParent (stale OnComponentBeginOverlap(InteractTrigger) _returnvalue))
    (Actor|Tick|SetActorTickEnabled false)))

(event EventInteract
  (bind _eventtoplayonfinish (Variables|Default|GetEventToPlayOnFinish))
  (if (Variables|Default|GetIsInteractable)
    (Widget|RemovefromParent (stale OnComponentBeginOverlap(InteractTrigger) _returnvalue))
    (bind _outactor (Sequencer|Player|CreateLevelSequencePlayer (Variables|Default|GetLevel%20Sequence)))
    (Sequencer|Player|Play (Variables|/Script/LevelSequence.LevelSequenceActor|GetSequencePlayer _outactor) :!class /Script/MovieScene.MovieSceneSequencePlayer)
    (if (Utilities|IsValid _eventtoplayonfinish)
      (Class|FMODBlueprintStatics|BusStopAllEvents "/Game/FMOD/Buses/Master/Music.Music" "ALLOWFADEOUT")
      (Class|FMODBlueprintStatics|PlayEventAttached _eventtoplayonfinish (Variables|/Script/Engine.PlayerCameraManager|GetTransformComponent (Game|GetPlayerCameraManager 0)) "None" "0, 0, 0" "KeepRelativeOffset"))))

(event EventTick
  (params (DeltaSeconds :type Float%20%28single-precision%29))
  (if (Utilities|IsValid (Variables|Default|GetWidget))
    (bind _asbp_player_pawnv_2 (Utilities|Casting|CastToBP_PlayerPawnv2 (Game|Player|GetPlayerPawn 0)))
    (if (Variables|/Script/GP3_Team03.GP3PlayerPawn|GetbIsUsingGamepad _asbp_player_pawnv_2)
      (Variables|/Game/Blueprints/Gameplay/BPWidget_Interact.BPWidget_Interact_C|SetInteract%20Texture (Variables|Default|GetWidget) (Variables|Default|Get'A'%20xbox%20icon))
      (else
        (Variables|/Game/Blueprints/Gameplay/BPWidget_Interact.BPWidget_Interact_C|SetInteract%20Texture (Variables|Default|GetWidget) (Variables|Default|Get'E'%20icon))))))

(event EventBeginPlay
  (Actor|Tick|SetActorTickEnabled false))

(fn ConstructionScript)