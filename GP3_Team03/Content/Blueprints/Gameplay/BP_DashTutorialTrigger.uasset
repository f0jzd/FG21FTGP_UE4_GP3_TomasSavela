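; BP_DashTutorialTrigger is a trigger volume that shows a dash tutorial widget while something overlaps its box.
; Overlap begin creates the TutorialDashWidget, plays its Dissolve animation in reverse and enables Tick, which is off at BeginPlay.
; While ticking, it reads IsUsingGamepad on BP_PlayerPawnv2 to switch the prompt texture between LB and Shift.
; Overlap end plays Dissolve forward and disables Tick, without removing the widget from the viewport.
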(event OnComponentBeginOverlap(Triggerbox)
  (params (OverlappedComponent :type Primitive%20Component%20Object%20Reference) (OtherActor :type Actor%20Object%20Reference) (OtherComp :type Primitive%20Component%20Object%20Reference) (OtherBodyIndex :type Integer) (bFromSweep :type Boolean) (SweepResult :type Hit%20Result%20Structure%20%28by%20ref%29))
  (bind _returnvalue (UserInterface|CreateWidget "/Game/Widgets/TutorialDashWidget.TutorialDashWidget_C"))
  (bind _output_get (Variables|Default|SetWidget _returnvalue))
  (UserInterface|Viewport|AddtoViewport _output_get 0)
  (UserInterface|Animation|PlayAnimation _output_get (Variables|/Game/Widgets/TutorialDashWidget.TutorialDashWidget_C|GetDissolve _output_get) 0.0 1 "Reverse" 1.0 false)
  (Actor|Tick|SetActorTickEnabled true))

(event OnComponentEndOverlap(Triggerbox)
  (params (OverlappedComponent :type Primitive%20Component%20Object%20Reference) (OtherActor :type Actor%20Object%20Reference) (OtherComp :type Primitive%20Component%20Object%20Reference) (OtherBodyIndex :type Integer))
  (bind _widget (Variables|Default|GetWidget))
  (UserInterface|Animation|PlayAnimation _widget (Variables|/Game/Widgets/TutorialDashWidget.TutorialDashWidget_C|GetDissolve _widget) 0.0 1 "Forward" 1.0 false)
  (Actor|Tick|SetActorTickEnabled false))

(event EventBeginPlay
  (Actor|Tick|SetActorTickEnabled false))

(event EventTick
  (params (DeltaSeconds :type Float%20%28single-precision%29))
  (if (Utilities|IsValid (Variables|Default|GetWidget))
    (bind _asbp_player_pawnv_2 (Utilities|Casting|CastToBP_PlayerPawnv2 (Game|Player|GetPlayerPawn 0)))
    (if (Variables|/Script/GP3_Team03.GP3PlayerPawn|GetbIsUsingGamepad _asbp_player_pawnv_2)
      (Variables|/Game/Widgets/TutorialDashWidget.TutorialDashWidget_C|SetDash%20Texture (Variables|Default|GetWidget) (Variables|Default|GetLB))
      (else
        (Variables|/Game/Widgets/TutorialDashWidget.TutorialDashWidget_C|SetDash%20Texture (Variables|Default|GetWidget) (Variables|Default|GetShift))))))

(fn ConstructionScript)