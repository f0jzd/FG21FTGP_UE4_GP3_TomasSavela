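; Sequence Director Blueprint for the Level 2 intro sequence, with two event-track callbacks that take player control away and later restore it.
; The first disables pawn input, then after a short delay hides the player widget, blocks pausing, and plays the Press_Play audio event attached to the camera manager with its Progress parameter set.
; The second re-enables input, the widget and pausing through the pawn reference cached by the first.
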(event Custom|SequenceEvent_0
  (bind _returnvalue (Game|Player|GetPlayerPawn 0))
  (Input|DisableInput _returnvalue 0)
  (Utilities|FlowControl|Delay 0.1)
  (bind _asbp_player_pawnv_2 (Utilities|Casting|CastToBP_PlayerPawnv2 _returnvalue))
  (Widget|SetVisibility (Variables|/Game/Blueprints/Player/BP_PlayerPawnv2.BP_PlayerPawnv2_C|GetPlayerWidget _asbp_player_pawnv_2) "Hidden")
  (Variables|/Game/Widgets/PauseMenuWidget.PauseMenuWidget_C|SetCanPause (Variables|/Game/Widgets/PlayerWidget.PlayerWidget_C|GetPauseMenuWidget (Variables|/Game/Blueprints/Player/BP_PlayerPawnv2.BP_PlayerPawnv2_C|GetPlayerWidget _asbp_player_pawnv_2)) false)
  (bind _returnvalue_2 (Class|FMODBlueprintStatics|PlayEventAttached "/Game/FMOD/Events/Music/Press_Play.Press_Play" (Variables|/Script/Engine.PlayerCameraManager|GetTransformComponent (Game|GetPlayerCameraManager 0)) "None" "0, 0, 0" "KeepRelativeOffset"))
  (Class|FMODAudioComponent|SetParameter _returnvalue_2 "Progress" 1.0))

(event Custom|SequenceEvent_1
  (Input|EnableInput (Game|Player|GetPlayerPawn 0) 0)
  (Widget|SetVisibility (Variables|/Game/Blueprints/Player/BP_PlayerPawnv2.BP_PlayerPawnv2_C|GetPlayerWidget (stale Custom|SequenceEvent_0 _asbp_player_pawnv_2)) "Visible")
  (Variables|/Game/Widgets/PauseMenuWidget.PauseMenuWidget_C|SetCanPause (Variables|/Game/Widgets/PlayerWidget.PlayerWidget_C|GetPauseMenuWidget (Variables|/Game/Blueprints/Player/BP_PlayerPawnv2.BP_PlayerPawnv2_C|GetPlayerWidget (stale Custom|SequenceEvent_0 _asbp_player_pawnv_2))) true))