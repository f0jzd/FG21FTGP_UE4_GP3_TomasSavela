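; Charge enemy character Blueprint that adds health display, state feedback and hitbox detection to the enemy.
; A widget health bar refreshes on BeginPlay and when the enemy takes gun damage, while state changes recolor an arrow component.
; Every tick the widget turns to face the first player controller's location with pitch locked at zero.
; HitboxCheck begin overlaps are forwarded to CallBegunOverlap.
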(event OnComponentBeginOverlap(HitboxCheck)
  (params (OverlappedComponent :type Primitive%20Component%20Object%20Reference) (OtherActor :type Actor%20Object%20Reference) (OtherComp :type Primitive%20Component%20Object%20Reference) (OtherBodyIndex :type Integer) (bFromSweep :type Boolean) (SweepResult :type Hit%20Result%20Structure%20%28by%20ref%29))
  (Default|CallBegunOverlap OtherActor))

(event Custom|UpdateHealth
  (Class|GP3ChargeEnemyHealth|UpdateHealth (.AsGP3%20Charge%20Enemy%20Health (Utilities|Casting|CastToGP3_ChargeEnemyHealth (UserInterface|GetWidget (Variables|Default|GetWidget)))) (Variables|Default|GetHealth)))

(event Custom|StateChanged_Event
  (params (New%20Clor :type Linear%20Color%20Structure))
  (Components|Arrow|SetArrowColor(LinearColor) (Variables|Default|GetArrow1) New%20Clor))

(event EventTick
  (params (DeltaSeconds :type Float%20%28single-precision%29))
  (bind _returnvalue (Transformation|GetActorLocation))
  (bind _returnvalue_2 (Game|GetPlayerController 0))
  (bind _returnvalue_3 (Transformation|GetActorLocation _returnvalue_2))
  (bind _returnvalue_4 (- _returnvalue_3 _returnvalue))
  (bind _returnvalue_5 (Math|Conversions|RotationFromXVector _returnvalue_4))
  (Transformation|SetWorldRotation (Variables|Default|GetWidget) (Math|Rotator|MakeRotator (.roll _returnvalue_5) 0.0 (.yaw _returnvalue_5)) false false))

(event EventBeginPlay
  (CallFunction|UpdateHealth)
  (EventDispatchers|BindEventtoStateChanged (delegate Custom|StateChanged_Event))
  (EventDispatchers|BindEventtoOnTookGunDamage (delegate Custom|UpdateHealth)))

(fn ConstructionScript)