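; Bull-like charging enemy that fades in and out with an erode material and runs a behavior tree once spawned.
; Player dash trails debuff it and show a weak-spot effect, cleared by timeout or a projectile hit there.
; Dashing through it deals damage with a short cooldown, while gun damage events refresh its player-facing health bar.
; Custom events supply audio, a charge curve and death, which stops AI and destroys it.
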(event OnComponentHit(WeakSpot)
  (params (HitComponent :type Primitive%20Component%20Object%20Reference) (OtherActor :type Actor%20Object%20Reference) (OtherComp :type Primitive%20Component%20Object%20Reference) (NormalImpulse :type Vector :default "0, 0, 0") (Hit :type Hit%20Result%20Structure%20%28by%20ref%29))
  (if (.bSuccess (Utilities|Casting|CastToBP_GunProjectile OtherActor))
    (if (Variables|Default|GetIsDebuffed)
      (Variables|Default|SetIsDebuffed false)
      (Components|Activation|Deactivate (Variables|Default|GetWeakpoint_exposed))
      (Components|Activation|Activate (Variables|Default|GetWeakspotHit) false))))

(event OnComponentBeginOverlap(Mesh)
  (params (OverlappedComponent :type Primitive%20Component%20Object%20Reference) (OtherActor :type Actor%20Object%20Reference) (OtherComp :type Primitive%20Component%20Object%20Reference) (OtherBodyIndex :type Integer) (bFromSweep :type Boolean) (SweepResult :type Hit%20Result%20Structure%20%28by%20ref%29))
  (bind (_asbp_player_pawnv_2 _bsuccess) (Utilities|Casting|CastToBP_PlayerPawnv2 OtherActor))
  (bind _dashcomp (Variables|/Script/GP3_Team03.GP3PlayerPawn|GetDashComp _asbp_player_pawnv_2))
  (if (not (Variables|Default|GetIsDead))
    (if (.bSuccess (Utilities|Casting|CastToGP3PlayerDashTrail OtherActor))
      (Variables|Default|SetDebuffTimeRemaining (Variables|Default|GetDebuff%20Duration))
      (Variables|Default|SetIsDebuffed true)
      (Default|CallIsDebuffedEvent)
      (elif _bsuccess
        (if (and (<= (Variables|Default|GetDashGracePeriod) 0.0) (Variables|/Script/GP3_Team03.GP3DashComponent|GetIsDashing _dashcomp))
          (Class|GP3AIBaseCharacter|TakeGunDamage (Variables|/Script/GP3_Team03.GP3DashComponent|GetDashDamage _dashcomp))
          (Variables|Default|SetDashGracePeriod 0.5)
          (Effects|SpawnEmitterAttached "/Game/3D_Art/Characters/Sanara_VFX/Impact/StarterContent/Particles/P_BulletHit.P_BulletHit" OverlappedComponent "None" "0, 0, 0" "0, 0, 0" "2.000000,2.000000,2.000000")
          (Class|FMODBlueprintStatics|PlayEventAttached "/Game/FMOD/Events/SFX_Player/Player_Dash_Through_Enemy.Player_Dash_Through_Enemy" OverlappedComponent "None" "0, 0, 0" "KeepRelativeOffset"))))))

(event Custom|ShowWeakspot
  (Components|Activation|Activate (Variables|Default|GetWeakpoint_exposed) false))

(event Custom|ChargeAudio
  ;[1 1 1] Charge Audio Event
  (Class|FMODBlueprintStatics|PlayEventAttached "/Game/FMOD/Events/SFX_Enemy/Bull/Enemy_Bull_Charging.Enemy_Bull_Charging" (Variables|Default|GetCapsuleComponent) "None" "0, 0, 0" "KeepRelativeOffset"))

(event Custom|StunAudio
  ;[1 1 1] Stun Audio Event
  (Class|FMODBlueprintStatics|PlayEventAttached "/Game/FMOD/Events/SFX_Enemy/Bull/Enemy_Bull_Charging.Enemy_Bull_Charging" (Variables|Default|GetCapsuleComponent) "None" "0, 0, 0" "KeepRelativeOffset"))

(event Custom|Timeline
  ;[1 1 1] Movement Curve Event
  (bind _floatchargecurve (Timeline|Timeline_0 PlayFromStart)
    (:Update
      (Variables|Default|SetTimelineCurveValue _floatchargecurve))))

(event Custom|Update%20Heath
  (CallFunction|UpdateHealthBar))

(event Custom|MovingAudio
  ;[1 1 1] Moving Audio Event
  (Utilities|FlowControl|Delay 0.4)
  (Class|FMODBlueprintStatics|PlayEventAttached "/Game/FMOD/Events/SFX_Enemy/Bull/Bull_Walking.Bull_Walking" (Variables|Default|GetCapsuleComponent) "None" "0, 0, 0" "KeepRelativeOffset"))

(event Custom|Activate%20Collision
  (Collision|SetCollisionEnabled (Variables|Character|GetMesh) "QueryAndPhysics")
  (Collision|SetCollisionEnabled (Variables|Default|GetWeakSpot) "QueryAndPhysics"))

(event Custom|CriticalDamage
  ;[1 1 1] CriticalDamage
  (Class|FMODBlueprintStatics|PlayEventatLocation "/Game/FMOD/Events/SFX_Enemy/Bull/Weakpoint_On_Damaged.Weakpoint_On_Damaged" (Transformation|GetActorTransform)))

(event EventTick
  (params (DeltaSeconds :type Float%20%28single-precision%29))
  (bind _returnvalue (Game|Player|GetPlayerPawn 0))
  (bind _returnvalue_2 (Transformation|GetActorLocation))
  (bind _returnvalue_3 (Transformation|GetActorLocation _returnvalue))
  (bind _returnvalue_4 (- _returnvalue_3 _returnvalue_2))
  (bind _returnvalue_5 (Math|Conversions|RotationFromXVector _returnvalue_4))
  (if (> (Variables|Default|GetDashGracePeriod) 0.0)
    (Variables|Default|SetDashGracePeriod (- (Variables|Default|GetDashGracePeriod) DeltaSeconds)))
  (if (<= 0.0 (Variables|Default|GetGracePeriod))
    (Variables|Default|SetGracePeriod (- (Variables|Default|GetGracePeriod) DeltaSeconds))
    (else
      (Variables|Default|SetIsOverlapping false)))
  (Transformation|SetWorldRotation (Variables|Default|GetHealthWidget) (Math|Rotator|MakeRotator (.roll _returnvalue_5) 0.0 (.yaw _returnvalue_5)) false false)
  (if (Collision|IsOverlappingActor (.AsGP3Player%20Dash%20Trail (Utilities|Casting|CastToGP3PlayerDashTrail (stale OnComponentBeginOverlap(Mesh) OtherActor))) :!class /Script/Engine.Actor)
    (Variables|Default|SetDebuffTimeRemaining (Variables|Default|GetDebuff%20Duration))
    (elif (< (Variables|Default|GetDebuffTimeRemaining) 0.0)
      (Variables|Default|SetIsDebuffed false)
      (Components|Activation|Deactivate (Variables|Default|GetWeakpoint_exposed))
      (else
        (Variables|Default|SetDebuffTimeRemaining (- (Variables|Default|GetDebuffTimeRemaining) DeltaSeconds))))))

(event EventBeginPlay
  (Rendering|SetVisibility (Variables|Default|GetHealthWidget) false false)
  (Transformation|AttachComponentToComponent (Variables|Default|GetWeakSpot) (Variables|Character|GetMesh) "HeadEnd" "KeepWorld" "KeepWorld" "KeepWorld" true)
  (Variables|Default|SetMaxHealth (Variables|Default|GetHealth))
  (bind _returnvalue (Rendering|Material|CreateDynamicMaterialInstance (Variables|Character|GetMesh) 0 "/Game/3D_Art/Characters/Monster_VFX/Death_Charger/Charge_01_Death_Mat.Charge_01_Death_Mat" "None" :!class /Script/Engine.PrimitiveComponent))
  (bind _output_get (Variables|Default|SetMaterial%20Instance _returnvalue))
  (bind _newtrack_0 (Timeline|Timeline_2 Play)
    (:Update
      (Rendering|Material|SetScalarParameterValue _output_get "Erode" _newtrack_0 :!class /Script/Engine.MaterialInstanceDynamic))
    (:Finished
      (Rendering|SetVisibility (Variables|Default|GetHealthWidget) true false)
      (CallFunction|UpdateHeath)
      (AI|RunBehaviorTree (AI|GetAIController (Pawn|GetController)) "/Game/Blueprints/AI/BehaviourTree/GP3BT_DefaultChargeBehaviour.GP3BT_DefaultChargeBehaviour")
      (CallFunction|ActivateCollision)
      (Components|Animation|PlayAnimation (Variables|Character|GetMesh) "/Game/3D_Art/Characters/Monster/Charge_01/Animations/Charger_01_Anim_Walk.Charger_01_Anim_Walk" true)
      (EventDispatchers|BindEventtoOnTookGunDamage (delegate Custom|Update%20Heath))
      (EventDispatchers|BindEventtoIsDebuffedEvent (delegate Custom|ShowWeakspot)))))

(event EventDeathAnimation
  ;[1 1 1] Death
  (CallFunction|OnDeath (Variables|Character|GetMesh))
  (EventDispatchers|UnbindEventfromOnTookGunDamage (delegate Custom|Update%20Heath))
  (EventDispatchers|UnbindEventfromIsDebuffedEvent (delegate Custom|ShowWeakspot))
  (Widget|SetVisibility (UserInterface|GetWidget (Variables|Default|GetHealthWidget)) "Hidden")
  (Class|FMODBlueprintStatics|PlayEventAttached "/Game/FMOD/Events/SFX_Enemy/Bull/Enemy_Bull_On_Death.Enemy_Bull_On_Death" (Variables|Default|GetCapsuleComponent) "None" "0, 0, 0" "KeepRelativeOffset")
  (if (Utilities|IsValid (Variables|Default|GetDashTrailRef))
    (Actor|DestroyActor (Variables|Default|GetDashTrailRef))
    (bind _newtrack_0 (Timeline|Timeline_1 Play)
      (:Update
        (Rendering|Material|SetScalarParameterValue (Variables|Default|GetMaterial%20Instance) "Erode" _newtrack_0 :!class /Script/Engine.MaterialInstanceDynamic))
      (:Finished
        (Actor|DestroyActor)))
    (else
      (Timeline|Timeline_1 Play))))

(fn ConstructionScript)

(fn SweepTest
  (bind _mesh (Variables|Character|GetMesh))
  (bind (_origin _boxextent) (Collision|GetComponentBounds _mesh))
  (Collision|BoxTraceByChannel (Transformation|GetActorLocation) _origin _boxextent (Transformation|GetActorRotation) "TraceTypeQuery1" false 0 "ForDuration" true "(R=1.000000,G=0.000000,B=0.000000,A=1.000000)" "(R=0.000000,G=1.000000,B=0.000000,A=1.000000)" 0.0)
  (return))

(fn OnDeath
  (params (self2 :type Skeletal%20Mesh%20Component%20Object%20Reference))
  (bind _self self)
  (bind _returnvalue (AI|GetAIController _self))
  (bind _asgp3bp_aiccharge_enemy (Utilities|Casting|CastToGP3BP_AICCharge_Enemy _returnvalue))
  (AI|Navigation|StopMovement _asgp3bp_aiccharge_enemy)
  (AI|Logic|StopLogic (Variables|/Script/AIModule.AIController|GetBrainComponent _asgp3bp_aiccharge_enemy) "Death")
  (Components|Animation|PlayAnimation self2 "/Game/3D_Art/Characters/Monster/Charge_01/Animations/Charger_01_Anim_Death_Hit_Effect.Charger_01_Anim_Death_Hit_Effect" false)
  (Variables|Default|SetIsDead true)
  (Variables|Default|SetDebuffTimeRemaining 0.0))

(fn SpawnFX
  (Development|PrintString "Hello"))

(fn UpdateHealthBar
  (bind _asbp_aihealth_widget (Utilities|Casting|CastToBP_AIHealthWidget (UserInterface|GetWidget (Variables|Default|GetHealthWidget))))
  (Progress|SetPercent (Variables|/Game/Blueprints/AI/AI_Widgets/BP_AIHealthWidget.BP_AIHealthWidget_C|GetProgressBar_0 _asbp_aihealth_widget) (Math|Float|NormalizetoRange (Variables|Default|GetHealth) 0.0 (Variables|Default|GetMaxHealth))))