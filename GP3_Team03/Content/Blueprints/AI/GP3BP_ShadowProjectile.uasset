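; Shadow projectile actor that explodes on reaching its target marker and damages the player within the blast radius.
; It attaches a Shadow_Ball particle system on BeginPlay and ignores sphere overlaps with anything other than TargetMarker.
; On impact, TookDamage scales Damage linearly down to zero at ExplosionRadius and passes it to the player's TakeExplosiveDamage.
; It then plays an explosion sound and destroys both the marker and itself.
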(event OnComponentBeginOverlap(Sphere)
  (params (OverlappedComponent :type Primitive%20Component%20Object%20Reference) (OtherActor :type Actor%20Object%20Reference) (OtherComp :type Primitive%20Component%20Object%20Reference) (OtherBodyIndex :type Integer) (bFromSweep :type Boolean) (SweepResult :type Hit%20Result%20Structure%20%28by%20ref%29))
  (bind _returnvalue (Transformation|GetActorLocation))
  (bind _targetmarker (Variables|Default|GetTargetMarker))
  (bind _playerref (Variables|Default|GetPlayerRef))
  (bind _returnvalue_2 (Transformation|GetActorLocation _playerref))
  (bind _returnvalue_3 (Math|Vector|Distance(Vector) _returnvalue_2 _returnvalue))
  (if (== OtherActor _targetmarker)
    (if (< _returnvalue_3 (Variables|Default|GetExplosionRadius))
      (CallFunction|TookDamage _returnvalue_3))
    ;[1 1 1] Explosion Sound Event
    (Class|FMODBlueprintStatics|PlayEventatLocation 0 (Transformation|GetActorTransform))
    (Actor|DestroyActor _targetmarker)
    (Actor|DestroyActor)))

(event EventBeginPlay
  (bind _scene (Variables|Default|GetScene))
  (Niagara|SpawnSystemAttached "/Game/3D_Art/Characters/Monster_VFX/Shadow_Ball_Ranged/Cast_Fire_Ball/shadow_Ball.shadow_Ball" _scene "None" (Variables|/Script/Engine.SceneComponent|GetRelativeLocation _scene) (Variables|/Script/Engine.SceneComponent|GetRelativeRotation _scene) "KeepRelativeOffset" false))

(fn ConstructionScript)

(fn TookDamage
  (params (DistanceFromCenter :type Float%20%28single-precision%29))
  (Class|GP3PlayerPawn|TakeExplosiveDamage (Variables|Default|GetPlayerRef) (* (/ (- (Variables|Default|GetExplosionRadius) DistanceFromCenter) (Variables|Default|GetExplosionRadius)) (Variables|Default|GetDamage)))
  (return))