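; Ranged mortar enemy character with health, a debuffable weak spot, a player-facing health bar and Wwise-style sound hooks.
; BeginPlay plays an erode-material spawn timeline, then enables collision, the behavior tree and debuff binding.
; Player dash trails open a timed weak spot, closed by projectile hits, while dashing through deals damage.
; Gun damage events update health; at zero, AI stops and the enemy erodes away before destruction.
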(event OnComponentHit(WeakSpot_0)
  (params (HitComponent :type Primitive%20Component%20Object%20Reference) (OtherActor :type Actor%20Object%20Reference) (OtherComp :type Primitive%20Component%20Object%20Reference) (NormalImpulse :type Vector :default "0, 0, 0") (Hit :type Hit%20Result%20Structure%20%28by%20ref%29))
  ;[1 1 1] Disable weakspot when hit
  (if (.bSuccess (Utilities|Casting|CastToBP_GunProjectile OtherActor))
    (if (Variables|Default|GetIsDebuffed)
      (Variables|Default|SetIsDebuffed false)
      (Components|Activation|Deactivate (Variables|Default|GetWeakspotVFX))
      (Components|Activation|Activate (Variables|Default|GetHitWeakspotVFX) false))))

(event OnComponentBeginOverlap(Box)
  (params (OverlappedComponent :type Primitive%20Component%20Object%20Reference) (OtherActor :type Actor%20Object%20Reference) (OtherComp :type Primitive%20Component%20Object%20Reference) (OtherBodyIndex :type Integer) (bFromSweep :type Boolean) (SweepResult :type Hit%20Result%20Structure%20%28by%20ref%29))
  (bind (_asbp_player_pawnv_2 _bsuccess) (Utilities|Casting|CastToBP_PlayerPawnv2 OtherActor))
  (bind _dashcomp (Variables|/Script/GP3_Team03.GP3PlayerPawn|GetDashComp _asbp_player_pawnv_2))
  (if (not (Variables|Default|GetIsDead))
    (if (.bSuccess (Utilities|Casting|CastToGP3PlayerDashTrail OtherActor))
      (if (<= (Variables|Default|GetBoxOverlapTimer) 0.0)
        (CallFunction|GotDebuff)
        (Variables|Default|SetIsDebuffed true)
        (Variables|Default|SetBoxOverlapTimer 1.0))
      (elif _bsuccess
        (if (and (Variables|/Script/GP3_Team03.GP3DashComponent|GetIsDashing _dashcomp) (<= (Variables|Default|GetDashGracePeriod) 0.0))
          (Class|GP3AIBaseCharacter|TakeGunDamage (Variables|/Script/GP3_Team03.GP3DashComponent|GetDashDamage _dashcomp))
          (Variables|Default|SetDashGracePeriod 0.5)
          (Effects|SpawnEmitterAttached "/Game/3D_Art/Characters/Sanara_VFX/Impact/StarterContent/Particles/P_BulletHit.P_BulletHit" OverlappedComponent "None" "0, 0, 0" "0, 0, 0" "2.000000,2.000000,2.000000")
          (Class|FMODBlueprintStatics|PlayEventAttached "/Game/FMOD/Events/SFX_Player/Player_Dash_Through_Enemy.Player_Dash_Through_Enemy" OverlappedComponent "None" "0, 0, 0" "KeepRelativeOffset"))))))

(event Custom|UpdateRangedHealth
  (CallFunction|UpdateHealthBar)
  (if (<= (Variables|Default|GetHealth) 0.0)
    (EventDispatchers|UnbindEventfromOnTookGunDamage (delegate Custom|UpdateRangedHealth))
    (CallFunction|Death)))

(event Custom|GotDebuff
  (Components|Activation|Activate (Variables|Default|GetWeakspotVFX) false)
  (Variables|Default|SetDebuffTimeRemaining (Variables|Default|GetDebuff%20Duration)))

(event Custom|Death
  (bind _self self)
  (bind _returnvalue (AI|GetAIController _self))
  (bind _asgp3bp_aicranged_enemy (Utilities|Casting|CastToGP3BP_AICRangedEnemy _returnvalue))
  (bind _braincomponent (Variables|/Script/AIModule.AIController|GetBrainComponent _asgp3bp_aicranged_enemy))
  (AI|Navigation|StopMovement _asgp3bp_aicranged_enemy)
  (if (Utilities|IsValid _braincomponent)
    (AI|Logic|StopLogic _braincomponent "Death"))
  ;[1 1 1] Death
  (Class|FMODBlueprintStatics|PlayEventAttached "/Game/FMOD/Events/SFX_Enemy/Mortar/Enemy_Mortar_On_Death.Enemy_Mortar_On_Death" (Variables|Default|GetEnemyShootingOrigin) "None" "0, 0, 0" "KeepRelativeOffset")
  (EventDispatchers|UnbindEventfromGotDebuffed (delegate Custom|GotDebuff))
  (Rendering|SetVisibility (Variables|Default|GetWidget_0) false false)
  (Components|Animation|PlayAnimation (Variables|Default|GetEnemyShootingOrigin) "/Game/3D_Art/Characters/Monster/Ranged_01/Animations/Ranged_01_AnimIdle_Death.Ranged_01_AnimIdle_Death" false)
  (Collision|SetCollisionEnabled (Variables|Default|GetWeakSpot_0) "NoCollision")
  (Collision|SetCollisionEnabled (Variables|Default|GetEnemyShootingOrigin) "NoCollision")
  (bind _newtrack_0 (Timeline|Timeline_0 Play)
    (:Update
      (Rendering|Material|SetScalarParameterValue (Variables|Default|GetMatieral%20Instance) "Erode" _newtrack_0 :!class /Script/Engine.MaterialInstanceDynamic))
    (:Finished
      (Actor|DestroyActor))))

(event Custom|CriticalDamage
  ;[1 1 1] TakeCriticalDamage
  (Class|FMODBlueprintStatics|PlayEventatLocation "/Game/FMOD/Events/SFX_Enemy/Mortar/Weakpoint_On_Damaged.Weakpoint_On_Damaged" (Transformation|GetActorTransform)))

(event Custom|Setup
  (EventDispatchers|BindEventtoOnTookGunDamage (delegate Custom|UpdateRangedHealth)))

(event Custom|Event%20RotateWidget
  ;[1 1 1] Rotate HP-bar widget event
  (CallFunction|SetWidgetRotation))

(event Custom|Activate%20Charge
  (Components|Activation|Activate (Variables|Default|GetChargingAttackVFX) false))

(event Custom|MarkAreaEvent
  (params (NewParam :type Transform))
  ;[1 1 1] Mark Area Sound
  (Class|FMODBlueprintStatics|PlayEventatLocation "/Game/FMOD/Events/SFX_Enemy/Mortar/Mortar_Marking_Impact_Area.Mortar_Marking_Impact_Area" NewParam))

(event Custom|Deactive%20Charge
  (Components|Activation|Deactivate (Variables|Default|GetChargingAttackVFX)))

(event Custom|AttackSound
  ;[1 1 1] AttackSound
  (Class|FMODBlueprintStatics|PlayEventAttached 0 (Variables|Default|GetEnemyShootingOrigin) "None" "0, 0, 0" "KeepRelativeOffset"))

(event Custom|ChargeAttack
  ;[1 1 1] ChargeAttack
  (Class|FMODBlueprintStatics|PlayEventAttached 0 (Variables|Default|GetEnemyShootingOrigin) "None" "0, 0, 0" "KeepRelativeOffset"))

(event EventTick
  (params (DeltaSeconds :type Float%20%28single-precision%29))
  (Variables|Default|SetBoxOverlapTimer (- (Variables|Default|GetBoxOverlapTimer) DeltaSeconds))
  (if (> (Variables|Default|GetDashGracePeriod) 0.0)
    (Variables|Default|SetDashGracePeriod (- (Variables|Default|GetDashGracePeriod) DeltaSeconds)))
  (CallFunction|EventRotateWidget)
  (CallFunction|CheckDebuffTime DeltaSeconds)
  ;[1 1 1] Mortar moving sound
  (Class|FMODBlueprintStatics|PlayEventAttached 0 (Variables|Default|GetEnemyShootingOrigin) "None" "0, 0, 0" "KeepRelativeOffset"))

(event EventBeginPlay
  (Rendering|SetVisibility (Variables|Default|GetWidget_0) false false)
  (Transformation|AttachComponentToComponent (Variables|Default|GetWeakSpot_0) (Variables|Default|GetEnemyShootingOrigin) "Chest" "KeepWorld" "KeepWorld" "KeepWorld" true)
  (Variables|Default|SetMaxHealth (Variables|Default|GetHealth))
  (CallFunction|Setup)
  (CallFunction|UpdateRangedHealth)
  (bind _returnvalue (Rendering|Material|CreateDynamicMaterialInstance (Variables|Default|GetEnemyShootingOrigin) 0 "/Game/3D_Art/Characters/Monster_VFX/Death_Ranged/Ranged_01_Spawn_Material_Inst.Ranged_01_Spawn_Material_Inst" "None" :!class /Script/Engine.PrimitiveComponent))
  (Variables|Default|SetMatieral%20Instance _returnvalue)
  (bind _newtrack_0 (Timeline|Timeline_1 Play)
    (:Update
      (Rendering|Material|SetScalarParameterValue (Variables|Default|GetMatieral%20Instance) "Erode" _newtrack_0 :!class /Script/Engine.MaterialInstanceDynamic))
    (:Finished
      (Rendering|SetVisibility (Variables|Default|GetWidget_0) true false)
      (Collision|SetCollisionEnabled (Variables|Default|GetEnemyShootingOrigin) "QueryOnly")
      (Collision|SetCollisionEnabled (Variables|Default|GetWeakSpot_0) "QueryAndPhysics")
      (AI|RunBehaviorTree (AI|GetAIController (Pawn|GetController)) "/Game/Blueprints/AI/BehaviourTree/GP3BT_DefaultRangedBehaviour.GP3BT_DefaultRangedBehaviour")
      (Components|Activation|Activate (Variables|Default|GetParticleSystem) false)
      (Components|Animation|PlayAnimation (Variables|Character|GetMesh) "/Game/3D_Art/Characters/Monster/Ranged_01/Animations/Ranged_01_AnimIdle.Ranged_01_AnimIdle" true)
      (Components|Animation|PlayAnimation (Variables|Default|GetEnemyShootingOrigin) "/Game/Blueprints/AI/GP3_RangedEnemyBlendSpace.GP3_RangedEnemyBlendSpace" false)
      (EventDispatchers|BindEventtoGotDebuffed (delegate Custom|GotDebuff)))))

(fn ConstructionScript)

(fn SetWidgetRotation
  (bind _returnvalue (Game|Player|GetPlayerPawn 0))
  (bind _returnvalue_2 (Transformation|GetActorLocation))
  (bind _returnvalue_3 (Transformation|GetActorLocation _returnvalue))
  (bind _returnvalue_4 (- _returnvalue_3 _returnvalue_2))
  (bind _returnvalue_5 (Math|Conversions|RotationFromXVector _returnvalue_4))
  (Transformation|SetWorldRotation (Variables|Default|GetWidget_0) (Math|Rotator|MakeRotator (.roll _returnvalue_5) 0.0 (.yaw _returnvalue_5)) false false)
  (return))

(fn CheckDebuffTime
  (params (Deltatime :type Float%20%28single-precision%29))
  (if (<= (Variables|Default|GetDebuffTimeRemaining) 0.0)
    (Components|Activation|Deactivate (Variables|Default|GetWeakspotVFX))
    (Variables|Default|SetIsDebuffed false)
    (else
      (Variables|Default|SetDebuffTimeRemaining (- (Variables|Default|GetDebuffTimeRemaining) Deltatime)))))

(fn UpdateHealthBar
  (bind _asbp_aihealth_widget (Utilities|Casting|CastToBP_AIHealthWidget (UserInterface|GetWidget (Variables|Default|GetWidget_0))))
  (Progress|SetPercent (Variables|/Game/Blueprints/AI/AI_Widgets/BP_AIHealthWidget.BP_AIHealthWidget_C|GetProgressBar_0 _asbp_aihealth_widget) (Math|Float|NormalizetoRange (Variables|Default|GetHealth) 0.0 (Variables|Default|GetMaxHealth))))